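; BP_Player is a 2D flipbook-animated player character that runs, jumps and punches via Enhanced Input.
; Movement swaps flipbooks and flips the sprite, is ignored mid-jump, and a Delay loop polls vertical velocity to detect landing.
; Attacking reveals a HitBox and damages overlapping BP_Human actors every tick until the sprite's finished-playing event resets it.
; Damage received is only printed.
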(event `self.ReceiveBeginPlay`
  ; Player movement
  (bind _asbp_player_controller (cast `/Game/Blueprints/BP_PlayerController` (`self.GetController`)))
  (`EnhancedInputSubsystemInterface.AddMappingContext` (pcsubsystem `EnhancedInputLocalPlayerSubsystem` _asbp_player_controller) "/Game/Blueprints/IMC_Default.IMC_Default" 0 (struct)))

(event `EnhancedInput|/Game/Blueprints/IA_Movement`
  (params (ActionValue :type "Float (double-precision)") (ElapsedSeconds :type "Float (double-precision)") (TriggeredSeconds :type "Float (double-precision)") (InputAction :type "InputAction Object Reference" :default "/Game/Blueprints/IA_Movement.IA_Movement"))
  ; Walking
  (:`Triggered`
    (if (not (`self.isJumping`))
      (`self.AddMovementInput` (`self.GetActorForwardVector`) ActionValue)
      (`PaperFlipbookComponent.SetFlipbook` (`self.Sprite`) "/Game/assets/run.run")
      (if (> ActionValue 0.0)
        (`SceneComponent.K2_SetWorldRotation` :`self` (`self.Sprite`))
        (else
          (`SceneComponent.K2_SetWorldRotation` (`self.Sprite`) (struct :`Yaw` -180.0) false false)))))
  (:`Completed`
    (if (not (`self.isJumping`))
      (`PaperFlipbookComponent.SetFlipbook` (`self.Sprite`) "/Game/assets/Idle.Idle"))))

(event `EnhancedInput|/Game/Blueprints/IA_Jump`
  (params (ActionValue :type Boolean) (ElapsedSeconds :type "Float (double-precision)") (TriggeredSeconds :type "Float (double-precision)") (InputAction :type "InputAction Object Reference" :default "/Game/Blueprints/IA_Jump.IA_Jump"))
  (bind _sprite (`self.Sprite`))
  ; Jumping
  (:`Triggered`
    (if (not (`self.isJumping`))
      (set `self.isJumping` true)
      (`self.Jump`)
      (`PaperFlipbookComponent.SetLooping` _sprite false)
      (`PaperFlipbookComponent.SetFlipbook` _sprite "/Game/assets/Jump.Jump")
      (`KismetSystemLibrary.Delay` 0.01)
      (if (== (.z (`self.GetVelocity`)) 0.0) :!label _label
        (`PaperFlipbookComponent.SetLooping` _sprite true)
        (`PaperFlipbookComponent.Play` _sprite)
        (`PaperFlipbookComponent.SetFlipbook` _sprite "/Game/assets/Idle.Idle")
        (set `self.isJumping` false)
        (else
          (`KismetSystemLibrary.Delay` 0.01)
          (goto _label))))))

(event `EnhancedInput|/Game/Blueprints/IA_Attack`
  (params (ActionValue :type Boolean) (ElapsedSeconds :type "Float (double-precision)") (TriggeredSeconds :type "Float (double-precision)") (InputAction :type "InputAction Object Reference" :default "/Game/Blueprints/IA_Attack.IA_Attack"))
  (:`Triggered`
    (`PaperFlipbookComponent.SetFlipbook` (`self.Sprite`) "/Game/assets/Attack.Attack")
    (`PaperFlipbookComponent.SetLooping` (`self.Sprite`) false)
    (set `self.IsPunching` true)
    (`SceneComponent.SetHiddenInGame` (`self.HitBox`) false false)))

(event `self.Sprite.OnFinishedPlaying`
  (bind _sprite (`self.Sprite`))
  (`PaperFlipbookComponent.SetFlipbook` _sprite "/Game/assets/Idle.Idle")
  (`PaperFlipbookComponent.SetLooping` _sprite true)
  (if (not (`PaperFlipbookComponent.IsPlaying` (`self.Sprite`)))
    (`PaperFlipbookComponent.Play` (`self.Sprite`))
    (set `self.IsPunching` false)
    (`SceneComponent.SetHiddenInGame` (`self.HitBox`) true false)))

(event `self.ReceiveTick`
  (params (DeltaSeconds :type "Float (single-precision)"))
  (if (`self.IsPunching`)
    (`self.HitCheck`)))

(event `self.ReceiveAnyDamage`
  (params (Damage :type "Float (single-precision)") (DamageType :type "DamageType Object Reference") (InstigatedBy :type "Controller Object Reference") (DamageCauser :type "Actor Object Reference"))
  (`KismetSystemLibrary.PrintString` (`KismetStringLibrary.Conv_DoubleToString` Damage)))

(fn `HitCheck`
  (for _array_element (`PrimitiveComponent.GetOverlappingActors` (`self.HitBox`) "/Game/Blueprints/BP_Human.BP_Human_C")
    (if (!= _array_element self)
      (`GameplayStatics.ApplyDamage` _array_element (`self.Damage Amount`) null null "/Script/Engine.DamageType")
      (else
        (`KismetSystemLibrary.PrintString` "No damage")))))

(fn `UserConstructionScript`)